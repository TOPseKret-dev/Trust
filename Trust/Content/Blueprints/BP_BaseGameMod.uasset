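; Base game mode that sets up two local players at tagged start points when play begins.
; BeginPlay caches all PlayerStart actors, then SpawnPlayers matches each player index to the start whose PlayerStartTag equals that number.
; For each match it creates the local player, spawns a BP_Char at the start's transform, has that controller possess it and records it in the Players array.
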(event `self.ReceiveBeginPlay`
  (bind _outactors (`GameplayStatics.GetAllActorsOfClass` "/Script/Engine.PlayerStart"))
  (set `self.StartPlayerArray` _outactors)
  (`self.SpawnPlayers`))

(fn `SpawnPlayers`
  (for _index (range 2)
    (set `self.index` _index)
    (for _array_element (`self.StartPlayerArray`)
      (if (== (`PlayerStart.PlayerStartTag` _array_element) (`KismetStringLibrary.Conv_IntToString` (`self.index`)))
        (`GameplayStatics.CreatePlayer` (`self.index`))
        (bind _returnvalue (`|SpawnActorFromClass` "/Game/Blueprints/BP_Char.BP_Char_C" (`self.GetTransform` _array_element) "Undefined" "OverrideRootScale" null null))
        (`Controller.Possess` (`GameplayStatics.GetPlayerController` (`self.index`)) _returnvalue)
        (`KismetArrayLibrary.Array_AddUnique` (`self.Players`) _returnvalue)))))

(fn `UserConstructionScript`)