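; BP_Camera is a shared camera that zooms in and out with the distance between two players.
; After a brief BeginPlay delay, ClassSetup takes both players from BP_BaseGameMod and makes this actor the view target for all PlayerControllers.
; A fast looping timer, used instead of Tick, sets the spring arm length to twice the player separation, clamped between minimum and maximum lengths.
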(event `self.ReceiveBeginPlay`
  (`KismetSystemLibrary.Delay` 0.001)
  (`self.ClassSetup`)
  (`KismetSystemLibrary.K2_SetTimer` null "UpdateCamera" 0.001 true))

(event `UpdateCamera`
  (set `SpringArmComponent.TargetArmLength` (`KismetMathLibrary.FClamp` (* (`self.GetDistanceTo` (`self.Player1`) (`self.Player2`)) 2.0) (`self.MinArmLength`) (`self.MaxArmLength`)) (`self.SpringArm`)))

(fn `ClassSetup`
  (bind _asbp_base_game_mod (cast `/Game/Blueprints/BP_BaseGameMod` (`GameplayStatics.GetGameMode`)))
  (bind _output_get (set `self.As BP Base Game Mod` _asbp_base_game_mod))
  (set `self.Players` (`/Game/Blueprints/BP_BaseGameMod.Players` _output_get))
  (bind _outactors (`GameplayStatics.GetAllActorsOfClass` "/Script/Engine.PlayerController"))
  (`PlayerController.SetViewTargetWithBlend` _outactors self 0.0 "VTBlend_Linear" 0.0 false)
  (set `self.Player1` (`|GetArrayItem` (`self.Players`)))
  (set `self.Player2` (`|GetArrayItem` (`self.Players`) 1)))

(fn `UserConstructionScript`)